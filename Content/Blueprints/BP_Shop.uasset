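; Shop Blueprint that offers four random weapons and four random upgrades, rerolled on a looping timer or through a refresh button.
; On BeginPlay it splits the item DataTable into per-type lists, creates the UI and adds the input mapping.
; One Enhanced Input action's value selects the held widget, and releasing it broadcasts the buy request.
; BP_PlayerTower's success or fail events then reroll the slot or whole shop, or show failure.
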(event Custom|OnShopUpdate
  ;[0.15 0.1064 0.04772 0.5] Automatic shop refresh
  (CallFunction|GetNewShop))

(event Custom|Event%20SuccessAction
  ;[0.08018 0.15 0.07523 0.5] On input action success
  (if (Variables|Refresh|GetIsRefreshButton)
    (CallFunction|GetNewShop)
    (Variables|Refresh|SetIsRefreshButton false)
    (Variables|Default|SetHeldWidget 0)
    (else
      (CallFunction|RefreshAfterBuy))))

(event Custom|Event%20FailAction
  ;[0.15 0.05308 0.05606 0.5] On input action fail
  (Default|DisplayBuyFail (Variables|Default|GetShopWidget))
  (Variables|Default|SetHeldWidget 0))

(event Input|EnhancedActionEvents|EnhancedInputActionIA_ShopSlot
  (params (ActionValue :type Float%20%28double-precision%29) (ElapsedSeconds :type Float%20%28double-precision%29) (TriggeredSeconds :type Float%20%28double-precision%29) (InputAction :type Input%20Action%20Object%20Reference :default "/Game/Inputs/IA_ShopSlot.IA_ShopSlot"))
  (bind _returnvalue (Math|Float|Truncate ActionValue))
  (bind _shopwidget (Variables|Default|GetShopWidget))
  (bind _shopwidget_2 (Variables|Default|GetShopWidget))
  (bind _shopwidget_3 (Variables|Default|GetShopWidget))
  (bind _returnvalue_2 (- _returnvalue 4))
  (bind _refresh (Variables|/Game/UI/WBP_Player.WBP_Player_C|GetRefresh _shopwidget_2))
  (bind _weaponsslots (Variables|/Game/UI/WBP_Player.WBP_Player_C|GetWeaponsSlots _shopwidget))
  (bind _upgradesslots (Variables|/Game/UI/WBP_Player.WBP_Player_C|GetUpgradesSlots _shopwidget_3))
  (bind _output (Utilities|Array|Get(acopy) _upgradesslots _returnvalue_2))
  (bind _output_2 (Utilities|Array|Get(acopy) _weaponsslots _returnvalue))
  ;[0.15 0.07734 0.07734 0.5] Manage shop inputs
  (:Triggered
    (Utilities|IsValid (Variables|Default|GetHeldWidget)
      (:Is%20Not%20Valid
        (if (<= ActionValue 7.0)
          (if (<= _returnvalue 3)
            (Default|OnHoldStart _output_2)
            (Variables|Default|SetHeldWidget _output_2)
            (else
              (Default|OnHoldStart _output)
              (Variables|Default|SetHeldWidget _output)))
          (else
            (Default|OnHoldStart _refresh)
            (Variables|Default|SetHeldWidget _refresh)
            (Variables|Refresh|SetIsRefreshButton true))))))
  (:Completed
    (Default|OnHoldEnd (Variables|Default|GetHeldWidget))
    (Default|CallOnItemBuy (Variables|/Game/UI/WBP_Icon.WBP_Icon_C|GetCurrentItem (Variables|Default|GetHeldWidget)))))

(event EventBeginPlay
  (bind _returnvalue (Game|GetPlayerController 0))
  (Utilities|FlowControl|Sequence
    (:then_0
      ;[0.1187 0.15 0.0875 0.5] Filling auxiliary arrays
      (Utilities|MakeTypeList (Variables|Default|GetItemsTable) (Variables|Lists|GetWeaponsList) "Weapon"
        (:End
          (Utilities|MakeTypeList (Variables|Default|GetItemsTable) (Variables|Lists|GetUpgradesList) "Upgrade"
            (:End
              ;[0.05271 0.1016 0.15 0.5] Adding shop UI to viewport
              (bind _returnvalue_2 (UserInterface|CreateWidget "/Game/UI/WBP_Player.WBP_Player_C" (Game|GetPlayerController 0)))
              (bind _output_get (Variables|Default|SetShopWidget _returnvalue_2))
              (UserInterface|Viewport|AddtoViewport _output_get 0)
              (Widget|SetVisibility _output_get "Visible")
              ;[0.15 0.1064 0.04772 0.5] Automatic shop refresh
              (CallFunction|OnShopUpdate)
              (bind _returnvalue_3 (Utilities|Time|SetTimerbyEvent (delegate Custom|OnShopUpdate) (Variables|Refresh|GetRefreshTime) true))
              (Variables|Refresh|SetRefreshHandle _returnvalue_3))))))
    (:then_1
      ;[0.06355 0.141 0.15 0.5] Adding mapping context
      (Input|AddMappingContext (PlayerController|LocalPlayerSubsystems|GetEnhancedInputLocalPlayerSubsystem _returnvalue) "/Game/Inputs/IMC_Shop.IMC_Shop" 0 "(bIgnoreAllPressedKeysUntilRelease=True,bForceImmediately=False,bNotifyUserSettings=False)")
      (Input|EnableInput _returnvalue))
    (:then_2
      ;[0.15 0.08969 0.1063 0.5] Binding external events
      (bind _returnvalue_4 (Actor|GetActorOfClass "/Game/Blueprints/BP_PlayerTower.BP_PlayerTower_C"))
      (bind _output_get_2 (Variables|Default|SetPlayer _returnvalue_4))
      (EventDispatchers|BindEventtoOnBuySuccess _output_get_2 (delegate Custom|Event%20SuccessAction))
      (EventDispatchers|BindEventtoOnBuyFail _output_get_2 (delegate Custom|Event%20FailAction)))))

(fn ConstructionScript)

(fn GetNewShop
  (for _index (range 0 3)
    (Utilities|FlowControl|Sequence
      (:then_0
        ;[0.15 0.07293 0.06695 0.5] Get new weapons set
        (bind _outitem (CallFunction|GetRandomItem "Weapon" (Variables|Lists|GetWeaponsList)))
        (Default|EventonShopUIUpdate (Variables|Default|GetShopWidget) "Weapon" _index _outitem))
      (:then_1
        ;[0.1336 0.15 0.08709 0.5] Get new upgrades set
        (bind _outitem_2 (CallFunction|GetRandomItem "Upgrade" (Variables|Lists|GetUpgradesList)))
        (Default|EventonShopUIUpdate (Variables|Default|GetShopWidget) "Upgrade" _index _outitem_2)))))

(fn GetRandomItem
  (params (Type :type EItemType%20Enum :default "None") (ItemsList :type Array%20of%20ST%20Items%20Structures))
  (bind _outitem (Utilities|Array|Random ItemsList))
  (bind (_type _upgradedata _weapondata) (Utilities|Struct|BreakST_Items _outitem))
  (switch Utilities|FlowControl|Switch|SwitchonEItemType Type
    (:Weapon
      (if (Utilities|IsValidSoftObjectReference _weapondata)
        (return _outitem)))
    (:Upgrade
      (if (Utilities|IsValidSoftObjectReference _upgradedata)
        (return _outitem)))))

(fn BuyItem
  (params (Item :type ST%20Items%20Structure))
  (if (and (> (.Price (Utilities|Struct|BreakST_Items Item)) 0) false)
    (Default|CallOnItemBuy)))

(fn RefreshAfterBuy
  (switch Utilities|FlowControl|Switch|SwitchonEItemType (.Type (Utilities|Struct|BreakST_Items (Variables|/Game/UI/WBP_Icon.WBP_Icon_C|GetCurrentItem (Variables|Default|GetHeldWidget))))
    (:Weapon
      (bind _outitem (CallFunction|GetRandomItem "None" (Variables|Lists|GetWeaponsList)))
      (bind _output_get (Variables|/Game/UI/WBP_Icon.WBP_Icon_C|SetCurrentItem (Variables|Default|GetHeldWidget) _outitem))
      (Default|Update (Variables|Default|GetHeldWidget) _output_get))
    (:Upgrade
      (bind _outitem_2 (CallFunction|GetRandomItem "None" (Variables|Lists|GetUpgradesList)))
      (bind _output_get_2 (Variables|/Game/UI/WBP_Icon.WBP_Icon_C|SetCurrentItem (Variables|Default|GetHeldWidget) _outitem_2))
      (Default|Update (Variables|Default|GetHeldWidget) _output_get_2)))
  (Variables|Default|SetHeldWidget 0))