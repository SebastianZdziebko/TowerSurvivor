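; Player tower Blueprint that handles purchases from BP_Shop, binding to its item-buy event on BeginPlay.
; Weapon buys check and charge the wallet component, add the weapon to the weapon system component, then signal success or failure.
; Upgrade logic covers income, defence and single-use stat-for-money trades through wallet and stats components.
; Upgrade purchasing is unfinished: only weapons are routed, and ApplyUpgrade is never called here.
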(event Custom|Event%20ManageBuy
  (params (Item :type ST%20Items%20Structure))
  ;[0.06436 0.05916 0.15 0.5] Manage buying process based on player's wallet status
  (switch Utilities|FlowControl|Switch|SwitchonEItemType (.Type (Utilities|Struct|BreakST_Items Item))
    (:Weapon
      (CallFunction|ManageWeaponBuy))))

(event EventBeginPlay
  ;[0.15 0.125 0.0417 0.5] Setup binds
  (bind _returnvalue (Actor|GetActorOfClass "/Game/Blueprints/BP_Shop.BP_Shop_C"))
  (Variables|Default|SetShop _returnvalue)
  (EventDispatchers|BindEventtoOnItemBuy _returnvalue (delegate Custom|Event%20ManageBuy)))

(fn ConstructionScript)

(fn ManageWeaponBuy
  (params (Item :type ST%20Items%20Structure%20%28by%20ref%29))
  (bind (_type _upgradedata _weapondata _weaponblueprint _price) (Utilities|Struct|BreakST_Items Item))
  (bind _returnvalue (Class|WalletComponent|CheckWallet (Variables|Default|GetWalletComp) _price))
  (if _returnvalue
    (Class|WalletComponent|RemovefromWallet (Variables|Default|GetWalletComp) _price)
    (Class|WeaponSystemComponent|AddWeapon (Variables|Default|GetWeaponSystemComp) _weaponblueprint)
    (Default|CallOnBuySuccess)
    (else
      (Default|CallOnBuyFail))))

(fn ManageUpgradeBuy
  (params (Item :type ST%20Items%20Structure))
  (bind (_type _upgradedata _weapondata _weaponblueprint _price) (Utilities|Struct|BreakST_Items Item))
  (if (and (Utilities|IsValidSoftObjectReference _upgradedata) (> _price 0))
    (bind _returnvalue (Class|WalletComponent|CheckWallet (Variables|Default|GetWalletComp) _price))
    (if _returnvalue
      (Class|WalletComponent|RemovefromWallet (Variables|Default|GetWalletComp) _price)
      (else
        (Default|CallOnBuyFail)))))

(fn ApplyUpgrade
  (params (Data :type Upgrade%20Data%20Object%20Reference))
  (bind _cost (Variables|/Script/TowerSurvivor.UpgradeData|GetCost Data))
  (bind _reward (Variables|/Script/TowerSurvivor.UpgradeData|GetReward Data))
  (bind _flatincome (Variables|/Script/TowerSurvivor.UpgradeData|GetFlatIncome Data))
  (bind _incomemodifier (Variables|/Script/TowerSurvivor.UpgradeData|GetIncomeModifier Data))
  (bind _changevalue (Variables|/Script/TowerSurvivor.UpgradeData|GetChangeValue Data))
  (switch Utilities|FlowControl|Switch|SwitchonEUpgradeType (Variables|/Script/TowerSurvivor.UpgradeData|GetType Data)
    (:Income
      ;[0.15 0.1382 0.03937 0.5] Income Upgrades
      (Utilities|FlowControl|Sequence
        (:then_0
          (if (> _flatincome 0)
            (Class|WalletComponent|IncreaseIncome (Variables|Default|GetWalletComp) _flatincome)))
        (:then_1
          (if (> _incomemodifier 0.0)
            (Class|WalletComponent|IncreaseIncomeModifier (Variables|Default|GetWalletComp) _incomemodifier)))))
    (:Defence
      ;[0.05577 0.07193 0.15 0.5] Defence Upgrade
      (if (> _changevalue 0)
        (Class|StatsComponent|IncreaseStat (Variables|Default|GetStatsComp) (Variables|/Script/TowerSurvivor.UpgradeData|GetStatType Data) _changevalue)))
    (:Single
      ;[0.15 0.05987 0.0494 0.5] Single Use
      (if (and (> _cost 0) (> _reward 0))
        (Class|StatsComponent|DecreaseStat (Variables|Default|GetStatsComp) (Variables|/Script/TowerSurvivor.UpgradeData|GetSpecialCostType Data) _cost)
        (Class|WalletComponent|AddtoWallet (Variables|Default|GetWalletComp) _reward)))))