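; BP_Swarm is a swarm enemy Blueprint whose logic here drives its health bar widget.
; On BeginPlay it caches the WB_EnemyHealthBar from its widget component and fills it.
; EnemyStatsComp's health update delegate then refreshes the bar through GetHealthPercentage_2, hiding it once the value is no longer above zero.
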(event OnHealthUpdateDelegate(EnemyStatsComp)
  (bind _returnvalue (|GetHealthPercentage_2))
  (bind _as_wb_enemy_health_bar (Variables|Default|GetAs%20WB%20Enemy%20Health%20Bar))
  ;[0.15 0.04843 0.04992 0.5] Update Health Bar when health changed
  (if (> _returnvalue 0.0)
    (Default|UpdateHealthBar _as_wb_enemy_health_bar _returnvalue)
    (else
      (Widget|SetVisibility _as_wb_enemy_health_bar "Hidden"))))

(event EventBeginPlay
  ;[0.08409 0.15 0.07655 0.5] Cast to Health Bar widget
  (bind _aswb_enemy_health_bar (Utilities|Casting|CastToWB_EnemyHealthBar (UserInterface|GetWidget (Variables|Default|GetHealthBarWidget))))
  (bind _output_get (Variables|Default|SetAs%20WB%20Enemy%20Health%20Bar _aswb_enemy_health_bar))
  ;[0.15 0.04843 0.04992 0.5] Comment
  (Default|UpdateHealthBar _output_get 1.0))

(fn ConstructionScript)