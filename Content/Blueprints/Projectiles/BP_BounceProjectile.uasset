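; Homing projectile that bounces from a hit enemy to others nearby until its bounces run out.
; Tick moves it toward its target; each hit runs parent logic, then searches around the victim and decrements the bounce count.
; The last hit spawns a Niagara effect and deactivates the trail system, delaying actor destruction until its particles finish.
; GetBounceRadius feeds the search, but its WeaponData.BounceRadius read is unconnected.
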(event OnSystemFinished(NiagaraComp)
  (params (PSystem :type Niagara%20Component%20Object%20Reference))
  ;[0.15 0.04655 0.02252 0.5] Destroy after all particles vanish
  (Actor|DestroyActor))

(event EventTick
  (params (DeltaSeconds :type Float%20%28single-precision%29))
  ;[0.15 0.1163 0.05336 0.5] Tick
  (Class|Projectile|MoveTowardsTarget DeltaSeconds))

(event EventBeginPlay
  ;[0.07021 0.0682 0.15 0.5] Setup
  (Collision|SetCollisionEnabled (Variables|Default|GetCollisionComp) "QueryOnly"))

(event EventOnProjectileDestroy
  (params (SpawnLocation :type Vector :default "0, 0, 0"))
  ;[0.15 0.114 0.1155 0.5] No bounces remaining
  (Niagara|SpawnSystematLocation (Variables|Default|GetHitEffect) SpawnLocation)
  (Components|Activation|Deactivate (Variables|Default|GetNiagaraComp)))

(event EventOnProjectileHit
  (params (OtherActor :type Actor%20Object%20Reference))
  (bind _returnvalue (Transformation|GetActorLocation OtherActor))
  ;[0.07371 0.15 0.08006 0.5] Hit targeted enemy
  (|CallParentFunction OtherActor)
  (if (> (Variables|Default|GetRemainingBouces) 0)
    (Class|Projectile|FindEnemyinRadius _returnvalue (|GetBounceRadius))
    (Math|Integer|DecrementInt (Variables|Default|GetRemainingBouces))
    (else
      (Class|Projectile|OnProjectileDestroy _returnvalue))))

(fn ConstructionScript)