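; Lightning projectile Blueprint that deals area damage on impact.
; BeginPlay runs the parent setup and pauses the Niagara effect until a hit.
; The first OnProjectileHit, gated by DoOnce, unpauses the effect and has Splash search around the hit actor, then damage any actors found, using radius and damage from WeaponData.
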(event EventBeginPlay
  ;[0.15 0.09828 0.08626 0.5] Setup
  (|CallParentFunction)
  (Class|NiagaraComponent|SetPaused (Variables|Default|GetNiagaraComp) true))

(event Collision|EventActorBeginOverlap
  (params (OtherActor :type Actor%20Object%20Reference)))

(event EventTick
  (params (DeltaSeconds :type Float%20%28single-precision%29))
  (|CallParentFunction DeltaSeconds) ; This node is disabled and will not be called.\nDrag off pins to build functionality.
)

(event EventOnProjectileHit
  (params (OtherActor :type Actor%20Object%20Reference))
  (bind _splash (Variables|Default|GetSplash))
  (bind _weapondata (Variables|Default|GetWeaponData))
  ;[0.1169 0.07485 0.15 0.5] Hit in AoE
  (Utilities|FlowControl|DoOnce false
    (:Completed
      (Class|NiagaraComponent|SetPaused (Variables|Default|GetNiagaraComp) false)
      (bind (_outactors _returnvalue) (Class|SplashComponent|SearchinSplashRadius _splash OtherActor (Variables|/Script/TowerSurvivor.WeaponData|GetSplashRadius _weapondata)))
      (if _returnvalue
        (Class|SplashComponent|DealDamageinSplash _splash _outactors (Variables|/Script/TowerSurvivor.WeaponData|GetDamage _weapondata))))))

(fn ConstructionScript)